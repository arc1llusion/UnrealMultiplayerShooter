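; Blueprint for the Blaster player character, adding overhead name display and debug-style key shortcuts.
; On BeginPlay it casts the OverheadWidget component's user widget to WPB_OverheadWidget and has it show this character's player name.
; Escape quits the game for the controlling player.
; Key 1, only with authority, casts the game mode to LobbyGameMode and calls GoToMainLevel to leave the lobby for the main level.
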(event `self.ReceiveBeginPlay`
  (bind _aswpb_overhead_widget (cast `/Game/Blueprints/HUD/WPB_OverheadWidget` (`WidgetComponent.GetUserWidgetObject` (`self.OverheadWidget`))))
  (`OverheadWidget.ShowPlayerName` _aswpb_overhead_widget self))

(event `Key|Escape`
  (params (Key :type "Key Structure"))
  (:`Pressed`
    (bind _asplayer_controller (cast `PlayerController` (`self.GetController` self)))
    (`KismetSystemLibrary.QuitGame` _asplayer_controller "Quit")))

(event `Key|One`
  (params (Key :type "Key Structure"))
  (:`Pressed`
    (if (`self.HasAuthority` self)
      (bind _aslobby_game_mode (cast `LobbyGameMode` (`GameplayStatics.GetGameMode`)))
      (if (`KismetSystemLibrary.IsValid` _aslobby_game_mode)
        (`LobbyGameMode.GoToMainLevel` _aslobby_game_mode)))))

(fn `UserConstructionScript`)